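; WallObstacle_BP is a wall obstacle that alters the main character's movement through two overlap boxes.
; Entering Box zeroes the character's velocity and gravity scale, suspending it in place, and leaving Box restores gravity scale to 1.
; Entering Box1 launches the character upward with a Z override at roughly 200 units, nudged by one if it is falling.
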(event `self.Box.OnComponentBeginOverlap`
  (params (OverlappedComponent :type "PrimitiveComponent Object Reference") (OtherActor :type "Actor Object Reference") (OtherComp :type "PrimitiveComponent Object Reference") (OtherBodyIndex :type Integer) (bFromSweep :type Boolean) (SweepResult :type "HitResult Structure (by ref)"))
  (bind _asmain_char_bp (cast `/Game/Blueprints/MainChar_BP` OtherActor))
  (bind (_returnvalue_x _returnvalue_y _returnvalue_z) (`KismetMathLibrary.BreakVector` (`self.GetVelocity` _asmain_char_bp)))
  (bind _charactermovement (`Character.CharacterMovement` _asmain_char_bp))
  (set `MovementComponent.Velocity` (`KismetMathLibrary.MakeVector` 0.0 0.0 (* 0 _returnvalue_z)) _charactermovement)
  (set `CharacterMovementComponent.GravityScale` 0.0 _charactermovement))

(event `self.Box1.OnComponentBeginOverlap`
  (params (OverlappedComponent :type "PrimitiveComponent Object Reference") (OtherActor :type "Actor Object Reference") (OtherComp :type "PrimitiveComponent Object Reference") (OtherBodyIndex :type Integer) (bFromSweep :type Boolean) (SweepResult :type "HitResult Structure (by ref)"))
  (bind _asmain_char_bp (cast `/Game/Blueprints/MainChar_BP` OtherActor))
  (bind (_velocity_x _velocity_y _velocity_z) (`KismetMathLibrary.BreakVector` (`MovementComponent.Velocity` (`Character.CharacterMovement` _asmain_char_bp))))
  (`Character.LaunchCharacter` _asmain_char_bp (`KismetMathLibrary.MakeVector` 0.0 0.0 (+ (`KismetMathLibrary.Conv_BoolToDouble` (< _velocity_z 0.0)) 200.0)) false true))

(event `self.Box.OnComponentEndOverlap`
  (params (OverlappedComponent :type "PrimitiveComponent Object Reference") (OtherActor :type "Actor Object Reference") (OtherComp :type "PrimitiveComponent Object Reference") (OtherBodyIndex :type Integer))
  (bind _asmain_char_bp (cast `/Game/Blueprints/MainChar_BP` OtherActor))
  (set `CharacterMovementComponent.GravityScale` 1.0 (`Character.CharacterMovement` _asmain_char_bp)))

(fn `UserConstructionScript`)
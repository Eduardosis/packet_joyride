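; Player character for a 2D side-scrolling flipbook game, with jump, double jump, mega jump and gravity-free air dash.
; DoOnce nodes gate each move and reset on landing.
; A looping timer raises the score widget each second, and AddPackage adds points, doubled during a timed power-up.
; It also detaches the camera at start, switches run/jump flipbooks on Tick, and opens pause and game-over widgets.
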(event `poweruptimer`
  (`/Engine/EditorBlueprintResources/StandardMacros.DoOnce` true :!label _label
    (:`Completed`
      (bind _output_get (set `self.contador` (`KismetMathLibrary.FClamp` (- (`self.contador`) (`GameplayStatics.GetWorldDeltaSeconds`)) 0.0 (`self.contador`))))
      (if (== _output_get 0.0)
        (set `self.isPoweredUp` false)))))

(event `self.ReceiveTick`
  (params (DeltaSeconds :type "Float (single-precision)"))
  ;[1 1 1] Handle animations
  (`|ExecutionSequence`
    (:`then_0`
      (`self.poweruptimer`))
    (:`then_1`
      (if (`self.isdead`)
        (`PaperFlipbookComponent.SetFlipbook` (`self.Sprite`) null)
        (elif (`NavMovementComponent.IsFalling` (`self.CharacterMovement`))
          (`PaperFlipbookComponent.SetFlipbook` (`self.Sprite`) "/Game/Astronaut/Character_jump.Character_jump")
          (else
            (`PaperFlipbookComponent.SetFlipbook` (`self.Sprite`) "/Game/Astronaut/Character_run.Character_run")))))))

(event `poweup`
  (set `self.isPoweredUp` true)
  (goto _label :!via `Reset`))

(event `self.ReceiveBeginPlay`
  (bind _returnvalue (`GameplayStatics.GetPlayerController` 0))
  ;[1 1 1] Event begin play events
  (set `PlayerController.bShowMouseCursor` false _returnvalue)
  (`WidgetBlueprintLibrary.SetInputMode_GameOnly` _returnvalue)
  (`SceneComponent.K2_DetachFromComponent` (`self.Camera`) "KeepWorld" "KeepWorld" "KeepWorld" true)
  (bind _returnvalue_2 (`|CreateWidget` "/Game/Blueprints/Score_BP.Score_BP_C"))
  (bind _output_get (set `self.Score` _returnvalue_2))
  (`UserWidget.AddToViewport` _output_get 0)
  (`KismetSystemLibrary.K2_SetTimerDelegate` (delegate `Update score`) 1.0 true))

(event `InputAction|Mega_Jump`
  (params (Key :type "Key Structure"))
  ;[1 1 1] Mega Jump
  (:`Pressed`
    (if (not (`self.isMegaJumping`))
      (`/Engine/EditorBlueprintResources/StandardMacros.DoOnce` false :!label _label_2
        (:`Completed`
          (set `self.isMegaJumping` true)
          (`self.LaunchCharacter` (0.0 0.0 1200.0) false true)
          (set `CharacterMovementComponent.GravityScale` 1.0 (`self.CharacterMovement`))
          (`KismetSystemLibrary.Delay` 1.0)
          (set `self.isMegaJumping` false))))))

(event `Update score`
  ;[1 1 1] Event begin play events
  (if (not (`self.isdead`))
    (bind _result (`/Engine/EditorBlueprintResources/StandardMacros.IncrementInt` (`self.scoreinteger`))
      (:`  `
        (`/Game/Blueprints/Score_BP.UpdateScore` (`self.Score`) _result)))))

(event `InputAction|Jump`
  (params (Key :type "Key Structure"))
  ;[1 1 1] Handle jumping
  (:`Pressed`
    (if (not (`self.isdead`))
      (`/Engine/EditorBlueprintResources/StandardMacros.DoOnce` false :!label _label_3
        (:`Completed`
          (`self.Jump`))))))

(event `InputAction|Jump`
  (params (Key :type "Key Structure"))
  (bind _charactermovement (`self.CharacterMovement`))
  ;[1 1 1] handle double jump
  (:`Pressed`
    (if (`NavMovementComponent.IsFalling` _charactermovement)
      (`/Engine/EditorBlueprintResources/StandardMacros.DoOnce` false :!label _label_4
        (:`Completed`
          (`self.LaunchCharacter` (0.0 0.0 300.0) false true)
          (set `CharacterMovementComponent.GravityScale` 1.0 _charactermovement))))))

(event `self.OnLanded`
  (params (Hit :type "HitResult Structure (by ref)"))
  (bind (_velocity_x _velocity_y _velocity_z) (`KismetMathLibrary.BreakVector` (`MovementComponent.Velocity` (`self.CharacterMovement`))))
  (bind _charactermovement (`Character.CharacterMovement` (`GameplayStatics.GetPlayerCharacter` 0)))
  ;[1 1 1] Handle jumping
  (`|ExecutionSequence`
    (:`then_0`
      (goto _label_3 :!via `Reset`))
    (:`then_1`
      (goto _label_5 :!via `Reset`))
    (:`then_2`
      (goto _label_4 :!via `Reset`))
    (:`then_3`
      (goto _label_2 :!via `Reset`))))

(event `InputAction|Dash`
  (params (Key :type "Key Structure"))
  (bind (_velocity_x _velocity_y _velocity_z) (`KismetMathLibrary.BreakVector` (`MovementComponent.Velocity` (`self.CharacterMovement`))))
  (bind _charactermovement (`Character.CharacterMovement` (`GameplayStatics.GetPlayerCharacter` 0)))
  ;[1 1 1] Dash event
  (:`Pressed`
    (if (`NavMovementComponent.IsFalling` (`self.CharacterMovement`))
      (if (not (`self.isDashing`))
        (`/Engine/EditorBlueprintResources/StandardMacros.DoOnce` false :!label _label_5
          (:`Completed`
            (set `self.isDashing` true)
            (`self.K2_SetActorLocation` (`GameplayStatics.GetPlayerCharacter` 0) (`CharacterMovementComponent.GetLastUpdateLocation` (`self.CharacterMovement`)) false false)
            (set `MovementComponent.Velocity` (`KismetMathLibrary.Conv_DoubleToVector` (* _velocity_z 0.0)) (`self.CharacterMovement`))
            (set `CharacterMovementComponent.GravityScale` 0.0 _charactermovement)
            (`KismetSystemLibrary.Delay` 0.75)
            (set `self.isDashing` false)
            (set `CharacterMovementComponent.GravityScale` 1.0 _charactermovement)))))))

(event `playerdead`
  ;[1 1 1] When player dies
  (set `self.isdead` true)
  (bind _returnvalue (`|CreateWidget` "/Game/Blueprints/Gameover_WBP.Gameover_WBP_C"))
  (`UserWidget.AddToViewport` _returnvalue 0)
  (`KismetSystemLibrary.Delay` 0.2)
  (`GameplayStatics.SetGamePaused` true))

(event `InputAction|Pause`
  (params (Key :type "Key Structure"))
  (bind _returnvalue (`GameplayStatics.GetPlayerController` 0))
  ;[1 1 1] Pause Game
  (:`Pressed`
    (`GameplayStatics.SetGamePaused` true)
    (bind _returnvalue_2 (`|CreateWidget` "/Game/pause/MenuPausa_WD.MenuPausa_WD_C"))
    (`UserWidget.AddToViewport` _returnvalue_2 0)
    (`WidgetBlueprintLibrary.SetInputMode_UIOnlyEx` _returnvalue null)
    (set `PlayerController.bShowMouseCursor` true _returnvalue)))

(event `InputAxis|MoveRight`
  (params (AxisValue :type "Float (single-precision)"))
  (`self.AddMovementInput` (1.0 0.0 0.0) AxisValue))

(fn `AddPackage`
  (if (`self.isPoweredUp`)
    (set `self.scoreinteger` (+ (`self.scoreinteger`) 2000))
    (else
      (set `self.scoreinteger` (+ (`self.scoreinteger`) 1000)))))

(fn `UserConstructionScript`)
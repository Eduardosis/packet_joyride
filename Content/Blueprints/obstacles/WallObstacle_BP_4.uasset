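; WallObstacle_BP_4 is a wall obstacle Blueprint holding leftover logic for altering MainChar_BP's vertical movement, none of which runs.
; Three disconnected chains each cast to MainChar_BP.
; One launches the character upward with Z override, another restores normal gravity, and the third zeroes velocity and gravity to suspend it.
; No event triggers these chains, and the construction script is empty.
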(fn `UserConstructionScript`)
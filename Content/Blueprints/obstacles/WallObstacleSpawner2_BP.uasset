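; WallObstacleSpawner2_BP is an obstacle spawner that periodically creates wall obstacles at its own scene transform.
; BeginPlay starts a looping timer with a random interval, rolled once, that fires SpawnRandomRock.
; Each tick picks a random integer, spawning WallObstacle_BP_4 on two of the three outcomes and nothing on the third.
; Spawn nodes for Packages_BP and other wall variants are left unconnected.
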(event `self.ReceiveBeginPlay`
  (`KismetSystemLibrary.K2_SetTimerDelegate` (delegate `Spawn random rock`) (`KismetMathLibrary.RandomFloatInRange` 0.5 5.0) true))

(event `Spawn random rock`
  (switch `int` (`KismetMathLibrary.RandomIntegerInRange` 0 2)
    (:`0`
      _)
    (:`1`
      _))
  (`|SpawnActorFromClass` "/Game/Blueprints/obstacles/WallObstacle_BP_4.WallObstacle_BP_4_C" (`SceneComponent.K2_GetComponentToWorld` (`self.Scene`)) "Undefined" "OverrideRootScale" null null))

(fn `UserConstructionScript`)
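; WallObstacle_BP_8 is a wall obstacle with two spike hazards and a collectible package for MainChar_BP.
; Overlapping either spike collision calls Playerdead on the character.
; Overlapping the capsule calls AddPackage on the character, then destroys the Package component through a DoOnce.
; AddPackage sits before the DoOnce, so the gate limits only the component's destruction.
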(event `self.spikescollision.OnComponentBeginOverlap`
  (params (OverlappedComponent :type "PrimitiveComponent Object Reference") (OtherActor :type "Actor Object Reference") (OtherComp :type "PrimitiveComponent Object Reference") (OtherBodyIndex :type Integer) (bFromSweep :type Boolean) (SweepResult :type "HitResult Structure (by ref)"))
  (bind _asmain_char_bp (cast `/Game/Blueprints/MainChar_BP` OtherActor))
  (`/Game/Blueprints/MainChar_BP.playerdead` _asmain_char_bp))

(event `self.spikescollision1.OnComponentBeginOverlap`
  (params (OverlappedComponent :type "PrimitiveComponent Object Reference") (OtherActor :type "Actor Object Reference") (OtherComp :type "PrimitiveComponent Object Reference") (OtherBodyIndex :type Integer) (bFromSweep :type Boolean) (SweepResult :type "HitResult Structure (by ref)"))
  (bind _asmain_char_bp (cast `/Game/Blueprints/MainChar_BP` OtherActor))
  (`/Game/Blueprints/MainChar_BP.playerdead` _asmain_char_bp))

(event `self.Capsule.OnComponentBeginOverlap`
  (params (OverlappedComponent :type "PrimitiveComponent Object Reference") (OtherActor :type "Actor Object Reference") (OtherComp :type "PrimitiveComponent Object Reference") (OtherBodyIndex :type Integer) (bFromSweep :type Boolean) (SweepResult :type "HitResult Structure (by ref)"))
  (bind _asmain_char_bp (cast `/Game/Blueprints/MainChar_BP` OtherActor))
  (`/Game/Blueprints/MainChar_BP.AddPackage` _asmain_char_bp)
  (`/Engine/EditorBlueprintResources/StandardMacros.DoOnce` false
    (:`Completed`
      (`ActorComponent.K2_DestroyComponent` (`self.package`)))))

(fn `UserConstructionScript`)